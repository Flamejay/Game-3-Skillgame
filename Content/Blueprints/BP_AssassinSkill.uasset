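; Pickup Assassin skill that attaches to the player on overlap and grants temporary invisibility, via material swap, and a speed boost.
; It only starts with an enemy inside DistanceCollision, and leaving range mid-skill ends it with a temporary slow and sprint lockout.
; Self-calling Delay events tick duration and cooldown, updating mana and stamina while active.
; Cooldown scales with duration used, and sounds and Niagara effects mark start and stop.
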(event `CheckDistance`
  (bind _outactors (`GameplayStatics.GetAllActorsOfClass` "/Game/AI_Blueprints/BP_Enemy_Base.BP_Enemy_Base_C"))
  (for _ _outactors
    _))

(event `self.HoldSkill`
  ;[1 1 1] Optional Event for skills that you'd like to "hold down".
  (if (`self.Skill is Active`)
    (bind _result (`/Engine/EditorBlueprintResources/StandardMacros.IncrementInt` (`self.HoldCount`))
      (:`  `
        (`KismetSystemLibrary.PrintString` (`KismetStringLibrary.Concat_StrStr` "This skill has been held down for " (`KismetStringLibrary.Conv_IntToString` _result) " frames.") true true (struct :`R` 1.0 :`G` 0.541323 :`A` 1.0) 0.0)))))

(event `self.EndSkill`
  ;[1 1 1] Optional, for skills that can be ended early.
  (`KismetSystemLibrary.Delay` 5.0)
  (`KismetSystemLibrary.PrintString` "Early End to BF Skill")
  (`self.Stop Skill`))

(event `self.BeginSkill`
  (bind _as_bp_third_person_character (`self.As BP Third Person Character`))
  (bind (_returnvalue_x _returnvalue_y) (`KismetMathLibrary.BreakVector` (`SceneComponent.K2_GetComponentLocation` (`self.DefaultSceneRoot`))))
  (bind _mesh (`Character.Mesh` _as_bp_third_person_character))
  ;[1 1 1] If the cooldown is at or below 0, we can start this skill!
  (if (`self.InRange`)
    (`KismetSystemLibrary.PrintString` "Begin BF Skill")
    (if (<= (`self.Skill Cooldown`) 0.0)
      (set `self.Skill is Active` true)
      (`GameplayStatics.PlaySoundAtLocation` "/Game/Audio/bleepbloops1.bleepbloops1" (`SceneComponent.K2_GetComponentLocation` (`self.DefaultSceneRoot`)) (struct) 1.0 1.0 0.0 null null null null)
      (`PrimitiveComponent.SetMaterial` _mesh 0 "/Game/Art/MM_Invisablity.MM_Invisablity")
      (`PrimitiveComponent.SetMaterial` _mesh 1 "/Game/Art/MM_Invisablity.MM_Invisablity")
      (set `CharacterMovementComponent.MaxWalkSpeed` 700.0 (`Character.CharacterMovement` _as_bp_third_person_character))
      (`NiagaraFunctionLibrary.SpawnSystemAtLocation` "/Game/Art/NS_InvisableEnter.NS_InvisableEnter" (`KismetMathLibrary.MakeVector` _returnvalue_x _returnvalue_y 125.0) (struct) (2.0 2.0 2.0))
      (`self.Update Skill Duration`))))

(event `Update Skill Duration`
  (bind _skill_duration (`self.Skill Duration`))
  ;[1 1 1] For every tenth of a second that this skill is active, reduce the number of remaining time on the skill.
  (if (`self.Skill is Active`)
    (bind _output_get (set `self.Skill Duration` (- _skill_duration 0.1)))
    (if (>= _skill_duration 0.0)
      (bind _isalive (`/Game/ThirdPerson/Blueprints/BP_ThirdPersonCharacter.Update Player Stats` (`self.As BP Third Person Character`) 0.0 -0.02 100.0))
      (if _isalive
        (`KismetSystemLibrary.Delay` 0.1)
        (`KismetSystemLibrary.PrintString` (`KismetStringLibrary.Concat_StrStr` "Assassin remaining duration  is" (`KismetStringLibrary.Conv_DoubleToString` _output_get)) true true (struct :`G` 0.66 :`B` 1.0 :`A` 1.0) 0.1)
        (`self.Update Skill Duration`)
        (else
          (`self.Stop SKill` :!label _label)))
      (else
        (goto _label)))))

(event `Stop Skill`
  (bind _as_bp_third_person_character (`self.As BP Third Person Character`))
  (bind (_returnvalue_x _returnvalue_y) (`KismetMathLibrary.BreakVector` (`SceneComponent.K2_GetComponentLocation` (`self.DefaultSceneRoot`))))
  (bind _mesh (`Character.Mesh` _as_bp_third_person_character))
  ;[1 1 1] Let's turn off the skill, either because the skill has run out of time, or because we have ended it early, or if the player has run out of mana
  (if (`self.Skill is Active`)
    (set `self.Skill is Active` false)
    (set `self.Skill Cooldown` (- 5.0 (`self.Skill Duration`))) ; subtract whatever time the \nplayer still had for this effect
    (set `self.Skill Duration` 5.0) ; reset skill duration
    (set `self.HoldCount` 0)
    (`GameplayStatics.PlaySoundAtLocation` "/Game/Audio/bleepbloops2.bleepbloops2" (`SceneComponent.K2_GetComponentLocation` (`self.DefaultSceneRoot`)) (struct) 1.0 1.0 0.0 null null null null)
    (`PrimitiveComponent.SetMaterial` _mesh 0 "/Game/Characters/Mannequins/Materials/Instances/Manny/MI_Manny_01.MI_Manny_01")
    (`PrimitiveComponent.SetMaterial` _mesh 1 "/Game/Materials/MI_LightGray.MI_LightGray")
    (set `CharacterMovementComponent.MaxWalkSpeed` 500.0 (`Character.CharacterMovement` _as_bp_third_person_character))
    (`NiagaraFunctionLibrary.SpawnSystemAtLocation` "/Game/Art/NS_InvisableExit.NS_InvisableExit" (`KismetMathLibrary.MakeVector` _returnvalue_x _returnvalue_y 125.0))
    (`self.Update Skill Cooldown`)
    (else
      (`KismetSystemLibrary.PrintString` "skill is already inactive"))))

(event `Update Skill Cooldown`
  ;[1 1 1] As long as Cooldown is above zero, let's reduce that number and stop the player from starting up this skill again.
  (if (> (`self.Skill Cooldown`) 0.0)
    (bind _output_get (set `self.Skill Cooldown` (- (`self.Skill Cooldown`) 0.1)))
    (`KismetSystemLibrary.Delay` 0.1)
    (`KismetSystemLibrary.PrintString` (`KismetStringLibrary.Concat_StrStr` "BrianDash cooldown is" (`KismetStringLibrary.Conv_DoubleToString` _output_get)) true true (struct :`G` 0.66 :`B` 1.0 :`A` 1.0) 0.1)
    (`self.Update Skill Cooldown`)))

(event `self.Sphere.OnComponentBeginOverlap`
  (params (OverlappedComponent :type "PrimitiveComponent Object Reference") (OtherActor :type "Actor Object Reference") (OtherComp :type "PrimitiveComponent Object Reference") (OtherBodyIndex :type Integer) (bFromSweep :type Boolean) (SweepResult :type "HitResult Structure (by ref)"))
  ;[1 1 1] grab the skill, unless we already have a skill
  (bind _asbp_third_person_character (cast `/Game/ThirdPerson/Blueprints/BP_ThirdPersonCharacter` OtherActor))
  (bind _output_get (set `self.As BP Third Person Character` _asbp_third_person_character)) ; We'll need this for mana, ammo, and other checks
  (`/Game/ThirdPerson/Blueprints/BP_ThirdPersonCharacter.CurrentSKill` _output_get
    (:`then`
      (`KismetSystemLibrary.PrintString` "You're already holding a skill!"))
    (:`else`
      (set `/Game/ThirdPerson/Blueprints/BP_ThirdPersonCharacter.CurrentSKill` self _output_get)
      (`self.K2_AttachToComponent` (`Character.Mesh` _output_get) "lhand" "SnapToTarget" "SnapToTarget" "SnapToTarget") ; attach this skill to the player's left hand
      (`self.K2_AttachToComponent` (`self.distanceCollision`) "spine_05" "SnapToTarget" "SnapToTarget" "SnapToTarget")
      (`KismetSystemLibrary.PrintString` "holding distance checker" true true (struct :`R` 1.0 :`B` 0.196342 :`A` 1.0) 3.0)
      (`GameplayStatics.PlaySoundAtLocation` "/Game/Audio/bleepbloops1.bleepbloops1" (`SceneComponent.K2_GetComponentLocation` (`self.DefaultSceneRoot`)) (struct) 1.0 1.0 0.0 null null null null)
      (`ActorComponent.K2_DestroyComponent` (`self.Sphere`))
      (`ActorComponent.K2_DestroyComponent` (`self.Cone`))
      (`ActorComponent.K2_DestroyComponent` (`self.TextRender`)))))

(event `self.distanceCollision.OnComponentBeginOverlap`
  (params (OverlappedComponent :type "PrimitiveComponent Object Reference") (OtherActor :type "Actor Object Reference") (OtherComp :type "PrimitiveComponent Object Reference") (OtherBodyIndex :type Integer) (bFromSweep :type Boolean) (SweepResult :type "HitResult Structure (by ref)"))
  (cast `/Game/AI_Blueprints/BP_Enemy_Base` OtherActor)
  (`KismetSystemLibrary.PrintString` "in Range" true true (struct :`G` 1.0 :`B` 0.0832 :`A` 1.0) 3.0)
  (set `self.InRange` true))

(event `self.distanceCollision.OnComponentEndOverlap`
  (params (OverlappedComponent :type "PrimitiveComponent Object Reference") (OtherActor :type "Actor Object Reference") (OtherComp :type "PrimitiveComponent Object Reference") (OtherBodyIndex :type Integer))
  (bind _as_bp_third_person_character (`self.As BP Third Person Character`))
  (bind _as_bp_third_person_character_2 (`self.As BP Third Person Character`))
  (cast `/Game/AI_Blueprints/BP_Enemy_Base` OtherActor)
  (`KismetSystemLibrary.PrintString` "Out of range" true true (struct :`R` 1.0 :`B` 0.091673 :`A` 1.0) 3.0)
  (set `self.InRange` false)
  (if (`self.Skill is Active`)
    (`self.Stop Skill`)
    (set `CharacterMovementComponent.MaxWalkSpeed` 100.0 (`Character.CharacterMovement` _as_bp_third_person_character_2))
    (set `SkeletalMeshComponent.GlobalAnimRateScale` 0.5 (`Character.Mesh` _as_bp_third_person_character_2))
    (set `/Game/ThirdPerson/Blueprints/BP_ThirdPersonCharacter.Stamina` 0.0 _as_bp_third_person_character_2)
    (set `/Game/ThirdPerson/Blueprints/BP_ThirdPersonCharacter.CanSprint` false _as_bp_third_person_character_2)
    (`KismetSystemLibrary.Delay` 4.0)
    (set `CharacterMovementComponent.MaxWalkSpeed` 500.0 (`Character.CharacterMovement` _as_bp_third_person_character))
    (set `SkeletalMeshComponent.GlobalAnimRateScale` 1.0 (`Character.Mesh` _as_bp_third_person_character))
    (set `/Game/ThirdPerson/Blueprints/BP_ThirdPersonCharacter.CanSprint` true _as_bp_third_person_character)))

(fn `UserConstructionScript`)